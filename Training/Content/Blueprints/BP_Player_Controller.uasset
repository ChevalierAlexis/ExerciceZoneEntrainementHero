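; Player controller that handles movement input, player stats and spell-targeting helpers for a third-person character.
; Input fires event dispatchers, with movement, look and jump handlers bound at BeginPlay; SpellCastEvent, not bound here, casts CurrentSpell.
; Clamped mana and PV, plus gold, update the W_UI widget.
; Summon and Throw trace from the follow camera to spawn actors or emitters, Throw returning overlapped actors; Tick restores grounded jump velocity after a delay.
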(event Custom|On_Turn_Event
  ;[1 1 1] Basic Controls
  (Pawn|Input|AddControllerYawInput (Game|GetPlayerCharacter 0) (stale Input|AxisEvents|InputAxisTurn AxisValue)))

(event Custom|OnMoveForwardEvent
  ;[1 1 1] Basic Controls
  (Pawn|Input|AddMovementInput (Game|GetPlayerCharacter 0) (Math|Vector|GetForwardVector (Math|Rotator|MakeRotator 0.0 0.0 (.Yaw (Math|Rotator|BreakRotator (Pawn|GetControlRotation :!class /Script/Engine.Controller))))) (stale Input|AxisEvents|InputAxisMoveForward AxisValue) false))

(event Custom|OnMoveRightEvent
  ;[1 1 1] Basic Controls
  (Pawn|Input|AddMovementInput (Game|GetPlayerCharacter 0) (Math|Vector|GetRightVector (Math|Rotator|MakeRotator 0.0 0.0 (.Yaw (Math|Rotator|BreakRotator (Pawn|GetControlRotation :!class /Script/Engine.Controller))))) (stale Input|AxisEvents|InputAxisMoveRight AxisValue) false))

(event Custom|OnJumpEvent
  ;[1 1 1] Basic Controls
  (Character|Jump (Game|GetPlayerCharacter 0)))

(event Custom|LookUpEvent
  ;[1 1 1] Basic Controls
  (Pawn|Input|AddControllerPitchInput (Game|GetPlayerCharacter 0) (stale Input|AxisEvents|InputAxisLookUp AxisValue)))

(event Custom|SpellCastEvent
  (bind _currentspell (Variables|Default|GetCurrentSpell))
  (if (!= _currentspell 0)
    (Default|CastSpell _currentspell self)))

(event EventTick
  (params (DeltaSeconds :type Float%20%28single-precision%29))
  (bind _returnvalue (Game|GetPlayerCharacter 0))
  (bind _charactermovement (Variables|/Script/Engine.Character|GetCharacterMovement _returnvalue))
  (if (not (AI|Components|NavMovement|IsFalling _charactermovement))
    (Utilities|FlowControl|Delay 1.0)
    (Variables|/Script/Engine.CharacterMovementComponent|SetJumpZVelocity _charactermovement 6e+02)))

(event EventBeginPlay
  (EventDispatchers|BindEventtoOnTurn (delegate Custom|On_Turn_Event))
  (EventDispatchers|BindEventtoOnJump (delegate Custom|OnJumpEvent))
  (EventDispatchers|BindEventtoOnMoveForward (delegate Custom|OnMoveForwardEvent))
  (EventDispatchers|BindEventtoOnMoveRight (delegate Custom|OnMoveRightEvent))
  (EventDispatchers|BindEventtoOnLookUp (delegate Custom|LookUpEvent))
  (bind _returnvalue (UserInterface|CreateWidget "/Game/Blueprints/W_UI.W_UI_C" self))
  (bind _output_get (Variables|Default|SetCurrentUI _returnvalue))
  (UserInterface|Viewport|AddtoViewport _output_get 0)
  (bind _asw_ui (Utilities|Casting|CastToW_UI _output_get))
  (Default|SetGoldText _asw_ui (Utilities|Text|ToText(Integer) (Variables|Default|GetGold)))
  (CallFunction|SetMana (Variables|Default|GetManaMax))
  (CallFunction|SetPV (Variables|Default|GetPVMax)))

(event Input|ActionEvents|InputActionCastSpell
  (params (Key :type Key%20Structure))
  (:Pressed
    (Default|CallOnSpellCast)))

(event Input|ActionEvents|InputActionJump
  (params (Key :type Key%20Structure))
  ;[1 1 1] Basic Controls
  (:Pressed
    (Default|CallOnJump)))

(event Input|AxisEvents|InputAxisLookUp
  (params (AxisValue :type Float%20%28single-precision%29))
  ;[1 1 1] Basic Controls
  (Default|CallOnLookUp))

(event Input|AxisEvents|InputAxisTurn
  (params (AxisValue :type Float%20%28single-precision%29))
  ;[1 1 1] Basic Controls
  (Default|CallOnTurn))

(event Input|AxisEvents|InputAxisMoveForward
  (params (AxisValue :type Float%20%28single-precision%29))
  ;[1 1 1] Basic Controls
  (Default|CallOnMoveForward))

(event Input|AxisEvents|InputAxisMoveRight
  (params (AxisValue :type Float%20%28single-precision%29))
  ;[1 1 1] Basic Controls
  (Default|CallOnMoveRight))

(fn ConstructionScript)

(fn SetMana
  (params (ManaAmount :type Integer))
  (Variables|Default|SetMana (Math|Integer|Clamp(Integer) (+ (Variables|Default|GetMana) ManaAmount) 0 (Variables|Default|GetManaMax)))
  (bind _asw_ui (Utilities|Casting|CastToW_UI (Variables|Default|GetCurrentUI)))
  (Default|SetManaBar _asw_ui (/ (Math|Conversions|ToFloat(Integer) (Variables|Default|GetMana)) (Math|Conversions|ToFloat(Integer) (Variables|Default|GetManaMax)))))

(fn SetPV
  (params (PVAmount :type Integer))
  (bind _output_get (Variables|Default|SetPV (Math|Integer|Clamp(Integer) (+ PVAmount (Variables|Default|GetPV)) 0 (Variables|Default|GetPVMax))))
  (bind _asw_ui (Utilities|Casting|CastToW_UI (Variables|Default|GetCurrentUI)))
  (Default|SetPvBar _asw_ui (/ (Math|Conversions|ToFloat(Integer) _output_get) (Math|Conversions|ToFloat(Integer) (Variables|Default|GetPVMax)))))

(fn SetGold
  (params (Price :type Integer))
  (Variables|Default|SetGold (- (Variables|Default|GetGold) Price))
  (bind _asw_ui (Utilities|Casting|CastToW_UI (Variables|Default|GetCurrentUI)))
  (Default|SetGoldText _asw_ui (Utilities|Text|ToText(Integer) (Variables|Default|GetGold))))

(fn Summon
  (params (Class :type Actor%20Class%20Reference))
  (bind _asbp_third_person_character (Utilities|Casting|CastToBP_ThirdPersonCharacter (Game|GetPlayerCharacter 0)))
  (bind _outhit (Collision|LineTraceByChannel (Transformation|GetWorldLocation (Variables|/Game/Blueprints/BP_ThirdPersonCharacter.BP_ThirdPersonCharacter_C|GetFollowCamera _asbp_third_person_character)) (+ (Transformation|GetWorldLocation (Variables|/Game/Blueprints/BP_ThirdPersonCharacter.BP_ThirdPersonCharacter_C|GetFollowCamera _asbp_third_person_character)) (* (Math|Vector|GetForwardVector (Variables|/Game/Blueprints/BP_ThirdPersonCharacter.BP_ThirdPersonCharacter_C|GetFollowCamera _asbp_third_person_character)) 2.5e+04)) "TraceTypeQuery2" false 0 "None"))
  (bind _returnvalue (Game|SpawnActorfromClass Class (Math|Conversions|ToTransform(Vector) (.location _outhit)) "Undefined" 0 0))
  (return _returnvalue))

(fn Throw
  (params (EmitterTemplate :type Particle%20System%20Object%20Reference))
  (bind _asbp_third_person_character (Utilities|Casting|CastToBP_ThirdPersonCharacter (Game|GetPlayerCharacter 0)))
  (bind _outhit (Collision|LineTraceByChannel (Transformation|GetWorldLocation (Variables|/Game/Blueprints/BP_ThirdPersonCharacter.BP_ThirdPersonCharacter_C|GetFollowCamera _asbp_third_person_character)) (+ (Transformation|GetWorldLocation (Variables|/Game/Blueprints/BP_ThirdPersonCharacter.BP_ThirdPersonCharacter_C|GetFollowCamera _asbp_third_person_character)) (* (Math|Vector|GetForwardVector (Variables|/Game/Blueprints/BP_ThirdPersonCharacter.BP_ThirdPersonCharacter_C|GetFollowCamera _asbp_third_person_character)) 2.5e+04)) "TraceTypeQuery1" false 0 "None"))
  (Effects|SpawnEmitteratLocation EmitterTemplate (.location _outhit))
  (bind (_outactors _returnvalue) (Collision|SphereOverlapActors (.location _outhit) 2e+03 (LocalVariables|GetObjectTypes) 0))
  (if _returnvalue
    (Development|PrintString "touché")
    (return _outactors)
    (else
      (Development|PrintString "Raté"))))