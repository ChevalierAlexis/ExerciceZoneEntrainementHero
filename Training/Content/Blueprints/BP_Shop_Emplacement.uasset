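; BP_Shop_Emplacement is a shop slot actor that sells a Product when the player walks into it.
; Text components show the product's name and price, set in both the construction script and BeginPlay.
; On actor overlap, it casts to BP_ThirdPersonCharacter and its BP_Player_Controller, then calls Buy on the Product with that controller.
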(event EventBeginPlay
  (bind _product (Variables|Default|GetProduct))
  (Rendering|Components|TextRender|SetText (Variables|Default|GetName) (Utilities|Text|ToText(String) (Variables|/Game/Blueprints/BP_DA_Products.BP_DA_Products_C|GetName _product)))
  (Rendering|Components|TextRender|SetText (Variables|Default|GetCost) (Utilities|Text|ToText(String) (Utilities|String|ToString(Integer) (Variables|/Game/Blueprints/BP_DA_Products.BP_DA_Products_C|GetPrice _product)))))

(event Collision|EventActorBeginOverlap
  (params (OtherActor :type Actor%20Object%20Reference))
  (bind _asthird_person_character (Utilities|Casting|CastToBP_ThirdPersonCharacter OtherActor))
  (bind _asbp_player_controller (Utilities|Casting|CastToBP_Player_Controller (Pawn|GetController _asthird_person_character)))
  (Default|Buy (Variables|Default|GetProduct) _asbp_player_controller))

(fn ConstructionScript
  (bind _product (Variables|Default|GetProduct))
  (Rendering|Components|TextRender|SetText (Variables|Default|GetName) (Utilities|Text|ToText(String) (Variables|/Game/Blueprints/BP_DA_Products.BP_DA_Products_C|GetName _product)))
  (Rendering|Components|TextRender|SetText (Variables|Default|GetCost) (Utilities|Text|ToText(String) (Utilities|String|ToString(Integer) (Variables|/Game/Blueprints/BP_DA_Products.BP_DA_Products_C|GetPrice _product)))))