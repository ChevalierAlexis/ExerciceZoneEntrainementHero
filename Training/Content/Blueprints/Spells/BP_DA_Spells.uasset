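; BP_DA_Spells is a base spell asset that can be bought and cast by the player.
; BuyEffect runs the parent effect, makes the spell the controller's CurrentSpell, binds an event to OnSpellCast and updates the UI spell image.
; CastSpell checks mana against the negated ManaCost, passes ManaCost to SetMana, then calls Action, an empty hook here, with the character and controller.
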(fn BuyEffect
  (params (Controller :type BP%20Player%20Controller%20Object%20Reference))
  (|CallParentFunction Controller)
  (Variables|/Game/Blueprints/BP_Player_Controller.BP_Player_Controller_C|SetCurrentSpell Controller self)
  (EventDispatchers|BindEventtoOnSpellCast Controller (EventDispatchers|CreateEvent Controller :!event SpellCastEvent))
  (bind _asw_ui (Utilities|Casting|CastToW_UI (Variables|/Game/Blueprints/BP_Player_Controller.BP_Player_Controller_C|GetCurrentUI Controller)))
  (Default|ChangeSpellImage _asw_ui (Variables|Default|GetImage)))

(fn Action
  (params (Character :type BP%20Third%20Person%20Character%20Object%20Reference) (Controller :type Player%20Controller%20Object%20Reference)))

(fn CastSpell
  (params (Controller :type Player%20Controller%20Object%20Reference))
  (bind _manacost (Variables|Default|GetManaCost))
  (bind _asbp_player_controller (Utilities|Casting|CastToBP_Player_Controller Controller))
  (if (>= (Variables|/Game/Blueprints/BP_Player_Controller.BP_Player_Controller_C|GetMana _asbp_player_controller) (- _manacost (* _manacost 2)))
    (Default|SetMana _asbp_player_controller (Variables|Default|GetManaCost))
    (bind _asbp_third_person_character (Utilities|Casting|CastToBP_ThirdPersonCharacter (Pawn|GetControlledPawn Controller)))
    (CallFunction|Action _asbp_third_person_character Controller)
    (else
      (Development|PrintString 0 "No Mana ?"))))